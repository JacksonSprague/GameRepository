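; SpaceshipTest is a spaceship actor that takes off once it has been activated three times and the sci-fi player character enters its trigger box.
; Each OnActivate call increments a counter and lights the next hidden point light, with the third lighting the last two.
; After a short delay, Tick moves the ship upward, compounding its speed every frame, so acceleration depends on frame rate.
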(event OnComponentBeginOverlap(Box)
  (params (OverlappedComponent :type Primitive%20Component%20Object%20Reference) (OtherActor :type Actor%20Object%20Reference) (OtherComp :type Primitive%20Component%20Object%20Reference) (OtherBodyIndex :type Integer) (bFromSweep :type Boolean) (SweepResult :type Hit%20Result%20Structure%20%28by%20ref%29))
  (Utilities|Casting|CastToBP_SciFiPlayer_Character OtherActor
    (:then
      (if (>= (Variables|Default|GetActivated) 3)
        (CallFunction|Launch)))
    (:CastFailed
      (Development|PrintString "none"))))

(event Custom|Launch
  (Utilities|FlowControl|Delay 0.2)
  (Variables|Default|SetLaunching true))

(event EventBeginPlay
  (Rendering|SetVisibility (Variables|Default|GetPointLight) false false)
  (Rendering|SetVisibility (Variables|Default|GetPointLight1) false false)
  (Rendering|SetVisibility (Variables|Default|GetPointLight2) false false)
  (Rendering|SetVisibility (Variables|Default|GetPointLight3) false false))

(event Collision|EventActorBeginOverlap
  (params (OtherActor :type Actor%20Object%20Reference)))

(event EventOnActivate
  (bind _result (Math|Integer|IncrementInt (Variables|Default|GetActivated))
    (:%20%20
      (if (== _result 1)
        (Rendering|SetVisibility (Variables|Default|GetPointLight) true false)
        (elif (== _result 2)
          (Rendering|SetVisibility (Variables|Default|GetPointLight1) true false)
          (elif (== _result 3)
            (Rendering|SetVisibility (Variables|Default|GetPointLight2) true false)
            (Rendering|SetVisibility (Variables|Default|GetPointLight3) true false)))))))

(event EventTick
  (params (DeltaSeconds :type Float%20%28single-precision%29))
  (bind _returnvalue (Transformation|GetActorLocation))
  (if (Variables|Default|GetLaunching)
    (Transformation|SetActorLocation (Math|Vector|MakeVector (.x _returnvalue) (.y _returnvalue) (+ (.z _returnvalue) (Variables|Default|Getcurrentspeed))) false false)
    (Variables|Default|Setcurrentspeed (* (Variables|Default|Getcurrentspeed) 1.005))))

(fn ConstructionScript)