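; BP_MessageLogLab is a message log actor with four constantly spinning meshes that shows text pages when interacted with.
; The construction script gives all four spinners one configurable mesh.
; OnInteract creates or reuses a textbox widget, advances through the Content array when allowed, flags the sci-fi player as Reading, then resets after the last entry.
; It exposes an interact prompt, while IsInteractable always returns false.
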(event EventTick
  (params (DeltaSeconds :type Float%20%28single-precision%29))
  ;[1 1 1] Spin
  (Transformation|AddWorldRotation (Variables|Default|GetSpinner) (Math|Rotator|MakeRotator 1.0 -1.5 2.0) false false)
  (Transformation|AddWorldRotation (Variables|Default|GetSpinner1) (Math|Rotator|MakeRotator -2.0 1.0 1.3) false false)
  (Transformation|AddWorldRotation (Variables|Default|GetSpinner2) (Math|Rotator|MakeRotator 1.0 -3.0 1.5) false false)
  (Transformation|AddWorldRotation (Variables|Default|GetSpinner3) (Math|Rotator|MakeRotator 2.0 -3.0 -1.7) false false))

(event EventBeginPlay
  ;[1 1 1] Begin
  (bind _asbp_sci_fi_player_character (Utilities|Casting|CastToBP_SciFiPlayer_Character (Game|GetPlayerCharacter 0))
    (:then
      (Variables|Default|SetPlayer_Ref _asbp_sci_fi_player_character))
    (:CastFailed
      (Development|PrintString "cast failed"))))

(event EventOnInteract
  (params (InteractingPlayer :type BP%20Sci%20Fi%20Player%20Character%20Object%20Reference))
  ;[1 1 1] Interact
  (Utilities|IsValid (Variables|Default|GetTextbox_UI)
    (:Is%20Valid
      _)
    (:Is%20Not%20Valid
      (bind _returnvalue (UserInterface|CreateWidget "/Game/Player/UI/TextBox.TextBox_C" (Game|GetPlayerController 0)))))
  (bind _output_get (Variables|Default|SetTextbox_UI _returnvalue))
  (UserInterface|Viewport|AddtoViewport _output_get 0)
  (if (Variables|/Game/Player/UI/TextBox.TextBox_C|GetCanAdvance (Variables|Default|GetTextbox_UI))
    (bind _result (Math|Integer|IncrementInt (Variables|Default|GetTalkIndex))
      (:%20%20
        (if (< _result (Utilities|Array|Length (Variables|Default|GetContent)))
          (Variables|/Game/Player/BP_SciFiPlayer_Character.BP_SciFiPlayer_Character_C|SetReading (Variables|Default|GetPlayer_Ref) true)
          (Default|PrintText (Variables|Default|GetTextbox_UI) (Utilities|Array|Get(acopy) (Variables|Default|GetContent) (Variables|Default|GetTalkIndex)))
          (else
            (Variables|/Game/Player/BP_SciFiPlayer_Character.BP_SciFiPlayer_Character_C|SetReading (Variables|Default|GetPlayer_Ref) false)
            (CallFunction|Reset)))))))

(fn ConstructionScript
  ;[1 1 1] Mesh
  (Components|StaticMesh|SetStaticMesh (Variables|Default|GetSphere) (Variables|Default|GetMesh))
  (Components|StaticMesh|SetStaticMesh (Variables|Default|GetSphere1) (Variables|Default|GetMesh))
  (Components|StaticMesh|SetStaticMesh (Variables|Default|GetSphere2) (Variables|Default|GetMesh))
  (Components|StaticMesh|SetStaticMesh (Variables|Default|GetSphere3) (Variables|Default|GetMesh)))

(fn Reset
  (Widget|RemovefromParent (Variables|Default|GetTextbox_UI))
  (Variables|Default|SetTalkIndex -1)
  (Variables|Default|SetTextbox_UI 0))

(fn InteractPrompt
  (return (Variables|Default|Getinteract%20prompt)))

(fn IsInteractable
  (return false))