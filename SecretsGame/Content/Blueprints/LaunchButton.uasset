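; LaunchButton is an interactable push button that activates the actor it controls.
; OnInteract plays a click sound and runs the Push timeline, which lowers Sphere1 slightly and sends OnActivateMessage to ControlledActor when it finishes.
; On BeginPlay the button attaches itself to ControlledActor, keeping its world transform.
; It supplies a "press" prompt, though IsInteractable always returns false.
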(event Custom|Press
  (bind _alpha (Timeline|Push' PlayFromStart)
    (:Update
      (Transformation|SetRelativeLocation (Variables|Default|GetSphere1) (Math|Vector|Lerp(Vector) "0.000000,0.000000,25.000000" "0.000000,0.000000,20.000000" _alpha) false false))
    (:Finished
      (Class|BPIElectricity|OnActivate(Message) (Variables|Default|GetControlledActor)))))

(event EventBeginPlay
  ;[1 1 1] Parent
  (Transformation|AttachActorToActor (Variables|Default|GetControlledActor) "None" "KeepWorld" "KeepWorld" "KeepWorld" true))

(event EventOnInteract
  (params (InteractingPlayer :type BP%20Sci%20Fi%20Player%20Character%20Object%20Reference))
  (CallFunction|Press)
  (Audio|PlaySound2D "/Game/SFX/simple_click.simple_click" 1.0 1.0 0.0 0 0))

(fn ConstructionScript)

(fn InteractPrompt
  (return "press"))

(fn IsInteractable
  (return false))