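; Interactable lever Blueprint that toggles an on/off state and relays it to a controlled actor.
; On interact, unless the Push timeline is playing, it plays a switch sound and runs the timeline forward or in reverse, rolling the lever between two angles.
; When the timeline finishes, its direction sets the On state, which is sent to ControlledActor through OnOffMessage.
; The prompt reads "press", though IsInteractable returns false.
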(event EventOnInteract
  (params (InteractingPlayer :type BP%20Sci%20Fi%20Player%20Character%20Object%20Reference))
  (if (not (Audio|Components|Audio|IsPlaying (Variables|Default|GetPush')))
    (Audio|PlaySound2D "/Game/SFX/LeverSwitch.LeverSwitch" 1.0 1.0 0.0 0 0)
    (if (not (Audio|Components|Audio|IsPlaying (Variables|Default|GetPush')))
      (if (Variables|Default|GetOn)
        (bind (_direction _alpha) (Timeline|Push' Reverse)
          (:Update
            (Transformation|SetRelativeRotation (Variables|Default|GetLever) (Math|Rotator|MakeRotator (Math|Float|Lerp 5e+01 -5e+01 _alpha) 0.0 0.0) false false))
          (:Finished
            (switch Utilities|FlowControl|Switch|SwitchonETimelineDirection _direction
              (:Forward
                (Variables|Default|SetOn true))
              (:Backward
                (Variables|Default|SetOn false)))
            (Class|BPIElectricity|On/Off(Message) (Variables|Default|GetControlledActor) (Variables|Default|GetOn))))
        (else
          (Timeline|Push' Play))))))

(fn ConstructionScript)

(fn InteractPrompt
  (return "press"))

(fn IsInteractable
  (return false))