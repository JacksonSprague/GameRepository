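; Launch code keypad terminal that lets the player enter a five-character code to authorize the ship's launch.
; CustomActivate appends each received command to the current code and shows it on a text render.
; Tick triggers a single check once five characters are entered, guarded by a flag.
; A match sets LaunchCodesAccurate on the ship reference, while a miss shows an error, then clears the entry for another try.
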(event Custom|Check
  (bind _textrender (Variables|Default|GetTextRender))
  (Utilities|FlowControl|Delay 0.2)
  (if (Utilities|Enum|Equal(Enum) (Variables|Default|GetCurrentCode) (Variables|Default|GetCorrectCode))
    (Rendering|Components|TextRender|SetText _textrender (Utilities|Text|ToText(String) "Correct!"))
    (Variables|/Game/Blueprints/SpaceshipTest.SpaceshipTest_C|SetLaunchCodesAccurate (Variables|Default|GetShip_Ref) true)
    (else
      (Rendering|Components|TextRender|SetText _textrender (Utilities|Text|ToText(String) "Incorrect"))
      (Utilities|FlowControl|Delay 1.5)
      (Variables|Default|SetCurrentCode "")
      (Rendering|Components|TextRender|SetText (Variables|Default|GetTextRender) (Utilities|Text|ToText(String) ""))
      (Variables|Default|SetCanCheck true))))

(event EventCustomActivate
  (params (command :type String))
  ;[1 1 1] Input
  (if (< (Utilities|String|Len (Variables|Default|GetCurrentCode)) 5)
    (bind _output_get (Variables|Default|SetCurrentCode (Utilities|String|Append (Variables|Default|GetCurrentCode) command)))
    (Rendering|Components|TextRender|SetText (Variables|Default|GetTextRender) (Utilities|Text|ToText(String) _output_get))))

(event EventTick
  (params (DeltaSeconds :type Float%20%28single-precision%29))
  ;[1 1 1] EventTick
  (if (== (Utilities|String|Len (Variables|Default|GetCurrentCode)) 5)
    (if (Variables|Default|GetCanCheck)
      (Variables|Default|SetCanCheck false)
      (CallFunction|Check))))

(fn ConstructionScript)