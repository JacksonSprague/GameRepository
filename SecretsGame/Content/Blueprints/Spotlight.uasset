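; Spotlight is a switchable light that reports its state to a referenced reactor as part of a code.
; Its On/Off event stores the state, shows or hides the RectLight and swaps the Sphere material between white emissive and black.
; Switching on adds the light's ID to the reactor's Code collection if absent, and switching off removes it.
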(event EventOn/Off
  (params (On? :type Boolean))
  (if On?
    (Rendering|SetVisibility (Variables|Default|GetRectLight) true false)
    (Variables|Default|SetOn true)
    (Rendering|Material|SetMaterial (Variables|Default|GetSphere) 0 "/Game/Materials/WhiteEmissive.WhiteEmissive")
    (if (not (Utilities|Array|ContainsItem (Variables|/Game/Blueprints/Reactor.Reactor_C|GetCode (Variables|Default|GetReactor_Ref)) (Variables|Default|GetID)))
      (Utilities|Array|Add (Variables|/Game/Blueprints/Reactor.Reactor_C|GetCode (Variables|Default|GetReactor_Ref)) (Variables|Default|GetID)))
    (else
      (Rendering|SetVisibility (Variables|Default|GetRectLight) false false)
      (Variables|Default|SetOn false)
      (Rendering|Material|SetMaterial (Variables|Default|GetSphere) 0 "/Game/Materials/Black.Black")
      (if (Utilities|Array|ContainsItem (Variables|/Game/Blueprints/Reactor.Reactor_C|GetCode (Variables|Default|GetReactor_Ref)) (Variables|Default|GetID))
        (Utilities|Array|RemoveItem (Variables|/Game/Blueprints/Reactor.Reactor_C|GetCode (Variables|Default|GetReactor_Ref)) (Variables|Default|GetID))))))

(fn ConstructionScript)