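; Bunker door actor that slides open and closed when activated.
; OnActivate toggles between Open and Close based on the IsOpen flag.
; A single timeline plays forward to open and reverses to close, lerping the Door component's relative location along X without sweep.
; IsInteractable always returns false, so the door does not report itself as interactable.
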(event Custom|Open
  ;[1 1 1] Animation
  (Variables|Default|SetIsOpen true)
  (bind _alpha (Timeline|T_Animation Play)
    (:Update
      (Transformation|SetRelativeLocation (Variables|Default|GetDoor) (Math|Vector|Lerp(Vector) "0.000000,0.000000,135.000000" "227.000000,0.000000,135.000000" _alpha) false false))))

(event Custom|Close
  ;[1 1 1] Animation
  (Variables|Default|SetIsOpen false)
  (bind _alpha (Timeline|T_Animation Reverse)
    (:Update
      (Transformation|SetRelativeLocation (Variables|Default|GetDoor) (Math|Vector|Lerp(Vector) "0.000000,0.000000,135.000000" "227.000000,0.000000,135.000000" _alpha) false false))))

(event EventOnActivate
  (if (Variables|Default|GetIsOpen)
    (CallFunction|Close)
    (else
      (CallFunction|Open))))

(fn ConstructionScript)

(fn IsInteractable
  (return false))