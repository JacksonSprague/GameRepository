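; Navigation dish that turns in 20-degree steps on Up, Down, Left and Right commands to align the ship's nav tower.
; CustomActivate changes the target angles, limiting only pitch, then a timeline lerps base yaw and head pitch.
; Each update sets the ship's NavTowerAligned flag by exact match to a fixed angle pair and prints rounded angles on the linked screen.
; CanMove blocks new commands until movement ends.
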(event EventCustomActivate
  (params (command :type String))
  (bind _ship_ref (Variables|Default|GetShip_Ref))
  ;[1 1 1] Custom Activate
  (if (Variables|Default|GetCanMove)
    (Variables|Default|SetCanMove false)
    ;[1 1 1] Checks
    (switch string command
      (:up
        (if (< (Variables|Default|GetVertical%20Degrees) 8e+01)
          ;[1 1 1] SetTarget
          (Variables|Default|SetVertical%20Degrees (+ (Variables|Default|GetVertical%20Degrees) 2e+01))
          ;[1 1 1] Initialize
          (Variables|Default|Setstartrotatehor (.yaw (Variables|/Script/Engine.SceneComponent|GetRelativeRotation (Variables|Default|GetBaseRotator))) :!label _label)
          (Variables|Default|Setstartrotatver (.pitch (Variables|/Script/Engine.SceneComponent|GetRelativeRotation (Variables|Default|GetHead%20Rotator))))
          ;[1 1 1] Rotate
          (bind _alpha (Timeline|TimelineLerp PlayFromStart)
            (:Update
              (Transformation|SetRelativeRotation (Variables|Default|GetBaseRotator) (Math|Rotator|MakeRotator 0.0 0.0 (Math|Float|Lerp (Variables|Default|Getstartrotatehor) (Variables|Default|GetHorizontalDegrees) _alpha)) false false)
              (Transformation|SetRelativeRotation (Variables|Default|GetHead%20Rotator) (Math|Rotator|MakeRotator 0.0 (Math|Float|Lerp (Variables|Default|Getstartrotatver) (Variables|Default|GetVertical%20Degrees) _alpha) 0.0) false false)
              (if (and (== (.yaw (Variables|/Script/Engine.SceneComponent|GetRelativeRotation (Variables|Default|GetBaseRotator))) 8e+01) (== (.pitch (Variables|/Script/Engine.SceneComponent|GetRelativeRotation (Variables|Default|GetHead%20Rotator))) 6e+01))
                (Variables|/Game/Blueprints/SpaceshipTest.SpaceshipTest_C|SetNavTowerAligned _ship_ref true)
                (else
                  (Variables|/Game/Blueprints/SpaceshipTest.SpaceshipTest_C|SetNavTowerAligned _ship_ref false)))
              ;[1 1 1] Screen
              (Rendering|Components|TextRender|SetText (Variables|/Game/Blueprints/TowerScreen.TowerScreen_C|GetTextRender (Variables|Default|GetScreen_Ref)) (Utilities|Text|ToText(String) (Utilities|String|Append (Utilities|String|Append (Utilities|String|Append (Utilities|String|ToString(Float) (Math|Conversions|ToFloat(Integer) (Math|Float|Round (.yaw (Variables|/Script/Engine.SceneComponent|GetRelativeRotation (Variables|Default|GetBaseRotator)))))) "0, ") (Utilities|String|ToString(Float) (Math|Conversions|ToFloat(Integer) (Math|Float|Round (.pitch (Variables|/Script/Engine.SceneComponent|GetRelativeRotation (Variables|Default|GetHead%20Rotator))))))) "0"))))
            (:Finished
              (Utilities|FlowControl|Delay 0.1)
              (Variables|Default|SetCanMove true)))
          (else
            (Variables|Default|SetCanMove true))))
      (:down
        (if (> (Variables|Default|GetVertical%20Degrees) 0.0)
          (Variables|Default|SetVertical%20Degrees (+ (Variables|Default|GetVertical%20Degrees) -2e+01))
          (goto _label)
          (else
            (Variables|Default|SetCanMove true))))
      (:left
        (Variables|Default|SetHorizontalDegrees (+ (Variables|Default|GetHorizontalDegrees) -2e+01))
        (goto _label))
      (:right
        (Variables|Default|SetHorizontalDegrees (+ (Variables|Default|GetHorizontalDegrees) 2e+01))
        (goto _label)))))

(fn ConstructionScript)