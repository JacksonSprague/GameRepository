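; Moving platform Blueprint that travels between StartCoords and EndCoords, driven by a trigger or an external command.
; The Movement timeline lerps the root's world location without sweep, and flips AtStart when it finishes.
; Overlapping Trig sends the platform to the opposite end, while CustomActivate, grouped as Electric, sends it to a commanded Start or End.
; Both inputs are ignored while the timeline is playing.
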(event OnComponentBeginOverlap(Trig)
  (params (OverlappedComponent :type Primitive%20Component%20Object%20Reference) (OtherActor :type Actor%20Object%20Reference) (OtherComp :type Primitive%20Component%20Object%20Reference) (OtherBodyIndex :type Integer) (bFromSweep :type Boolean) (SweepResult :type Hit%20Result%20Structure%20%28by%20ref%29))
  ;[1 1 1] Movement
  (if (not (Audio|Components|Audio|IsPlaying (Variables|Default|GetMovement)))
    (if (Variables|Default|GetAtStart)
      (bind _movement (Timeline|Movement PlayFromStart)
        (:Update
          (Transformation|SetWorldLocation (Variables|Default|GetDefaultSceneRoot) (Math|Vector|Lerp(Vector) (Variables|Default|GetStartCoords) (Variables|Default|GetEndCoords) _movement) false false))
        (:Finished
          (Variables|Default|SetAtStart (not (Variables|Default|GetAtStart)))))
      (else
        (Timeline|Movement ReverseFromEnd)))))

(event EventBeginPlay)

(event EventCustomActivate
  (params (command :type String))
  ;[1 1 1] Electric
  (if (not (Audio|Components|Audio|IsPlaying (Variables|Default|GetMovement)))
    (switch string command
      (:Start
        (if (not (Variables|Default|GetAtStart))
          ;[1 1 1] Movement
          (bind _movement (Timeline|Movement ReverseFromEnd)
            (:Update
              (Transformation|SetWorldLocation (Variables|Default|GetDefaultSceneRoot) (Math|Vector|Lerp(Vector) (Variables|Default|GetStartCoords) (Variables|Default|GetEndCoords) _movement) false false))
            (:Finished
              (Variables|Default|SetAtStart (not (Variables|Default|GetAtStart)))))))
      (:End
        (if (Variables|Default|GetAtStart)
          (Timeline|Movement PlayFromStart))))))

(fn ConstructionScript)