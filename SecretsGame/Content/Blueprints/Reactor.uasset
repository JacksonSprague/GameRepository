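; Reactor Blueprint that powers up the ship when activated with a valid fuel code, otherwise printing an unstable-fuel warning.
; Check tests which numbers the Code collection contains before Activate runs.
; Chained timelines raise the core and scale up its cones, then Tick spins them with exponentially increasing, clamped speed.
; After a delay it marks itself active, gives the ship power and sends the door an activate message.
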(event Custom|Activate
  ;[1 1 1] Ready
  (bind _newtrack_0 (Timeline|Raise PlayFromStart)
    (:Update
      (Transformation|SetRelativeLocation (Variables|Default|GetReactorCore) (Math|Vector|Lerp(Vector) "0.000000,0.000000,300.000000" "0.000000,0.000000,450.000000" _newtrack_0) false false))
    (:Finished
      (Utilities|FlowControl|Delay 1.0)
      (bind _newtrack_0_2 (Timeline|Extend PlayFromStart)
        (:Update
          (Transformation|SetRelativeScale3D (Variables|Default|GetConesCore) (Math|Vector|Lerp(Vector) "0.400000,0.400000,0.400000" "0.800000,0.800000,0.800000" _newtrack_0_2)))
        (:Finished
          (Variables|Default|SetSpin true)
          (Utilities|FlowControl|Delay 5.0)
          (Variables|Default|SetActive true)
          (Variables|/Game/Blueprints/SpaceshipTest.SpaceshipTest_C|SetHasPower (Variables|Default|GetShip_Ref) true)
          (Class|BPIElectricity|OnActivate(Message) (Variables|Default|GetDoor)))))))

(event EventTick
  (params (DeltaSeconds :type Float%20%28single-precision%29))
  (bind _conescore (Variables|Default|GetConesCore))
  (bind _returnvalue (Transformation|GetWorldRotation _conescore))
  ;[1 1 1] Spin
  (if (Variables|Default|GetSpin)
    (Transformation|SetWorldRotation _conescore (Math|Rotator|MakeRotator (+ (.roll _returnvalue) (/ (Variables|Default|Getrotatespeed) 2.0)) (.pitch _returnvalue) (+ (.yaw _returnvalue) (Variables|Default|Getrotatespeed))) false false)
    (Variables|Default|Setrotatespeed (Math|Float|Clamp(Float) (* (Variables|Default|Getrotatespeed) 1.005) 0.0 5e+01))))

(event EventOnActivate
  ;[1 1 1] BPI
  (bind _ready (CallFunction|Check))
  (if _ready
    (CallFunction|Activate)
    (else
      (Development|PrintString "Fuel unstable"))))

(fn ConstructionScript)

(fn Check
  (return (Math|Boolean|ANDBoolean (not (Utilities|Array|ContainsItem (Variables|Default|GetCode) 0)) (Utilities|Array|ContainsItem (Variables|Default|GetCode) 1) (Utilities|Array|ContainsItem (Variables|Default|GetCode) 2) (not (Utilities|Array|ContainsItem (Variables|Default|GetCode) 3)) (Utilities|Array|ContainsItem (Variables|Default|GetCode) 4) (not (Utilities|Array|ContainsItem (Variables|Default|GetCode) 5)) (Utilities|Array|ContainsItem (Variables|Default|GetCode) 6))))