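; Shy_Door is a door that vanishes and lets pawns through while the player is inside its DetectZone with ShyEnable off.
; Zone overlaps set the door's Detect flag and mirror it to ShyDetect on the cached sci-fi player character.
; Tick polls both flags to set Active, visibility and Pawn collision, keeping the door solid in every other case.
; IsInteractable always returns false.
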(event OnComponentBeginOverlap(DetectZone)
  (params (OverlappedComponent :type Primitive%20Component%20Object%20Reference) (OtherActor :type Actor%20Object%20Reference) (OtherComp :type Primitive%20Component%20Object%20Reference) (OtherBodyIndex :type Integer) (bFromSweep :type Boolean) (SweepResult :type Hit%20Result%20Structure%20%28by%20ref%29))
  ;[1 1 1] DetectZone
  (if (== OtherActor (Variables|Default|GetAs%20BP%20Sci%20Fi%20Player%20Character))
    (Variables|Default|SetDetect true)
    (Variables|/Game/Player/BP_SciFiPlayer_Character.BP_SciFiPlayer_Character_C|SetShyDetect (Variables|Default|GetAs%20BP%20Sci%20Fi%20Player%20Character) true)))

(event OnComponentEndOverlap(DetectZone)
  (params (OverlappedComponent :type Primitive%20Component%20Object%20Reference) (OtherActor :type Actor%20Object%20Reference) (OtherComp :type Primitive%20Component%20Object%20Reference) (OtherBodyIndex :type Integer))
  ;[1 1 1] DetectZone
  (if (== OtherActor (Variables|Default|GetAs%20BP%20Sci%20Fi%20Player%20Character))
    (Variables|Default|SetDetect false)
    (Variables|/Game/Player/BP_SciFiPlayer_Character.BP_SciFiPlayer_Character_C|SetShyDetect (Variables|Default|GetAs%20BP%20Sci%20Fi%20Player%20Character) false)))

(event EventTick
  (params (DeltaSeconds :type Float%20%28single-precision%29))
  (bind _door (Variables|Default|GetDoor))
  (bind _door_2 (Variables|Default|GetDoor))
  (bind _door_3 (Variables|Default|GetDoor))
  ;[1 1 1] Detect
  (if (Variables|Default|GetDetect)
    (if (Variables|/Game/Player/BP_SciFiPlayer_Character.BP_SciFiPlayer_Character_C|GetShyEnable (Variables|Default|GetAs%20BP%20Sci%20Fi%20Player%20Character))
      (Variables|Default|SetActive true)
      (Rendering|SetVisibility _door_3 true true)
      (Collision|SetCollisionResponsetoChannel _door_3 "ECC_Pawn" "ECR_Block")
      (else
        (Variables|Default|SetActive false)
        (Rendering|SetVisibility _door_2 false true)
        (Collision|SetCollisionResponsetoChannel _door_2 "ECC_Pawn" "ECR_Ignore")))
    (else
      (Variables|Default|SetActive true)
      (Rendering|SetVisibility _door true true)
      (Collision|SetCollisionResponsetoChannel _door "ECC_Pawn" "ECR_Block"))))

(event EventBeginPlay
  ;[1 1 1] BeginPlay
  (bind _asbp_sci_fi_player_character (Utilities|Casting|CastToBP_SciFiPlayer_Character (Game|GetPlayerCharacter 0)))
  (Variables|Default|SetAs%20BP%20Sci%20Fi%20Player%20Character _asbp_sci_fi_player_character))

(fn ConstructionScript)

(fn IsInteractable
  (return false))