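; BP_MessageLog is an interactable message source that shows its Content entries one at a time in a TextBox widget.
; Each OnInteract creates the widget if needed, adds it to the viewport and, when it can advance, increments TalkIndex to print the next entry.
; Past the last entry, Reset removes the widget and rewinds the index.
; IsInteractable always returns false here.
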(event EventOnInteract
  (params (InteractingPlayer :type BP%20Sci%20Fi%20Player%20Character%20Object%20Reference))
  (Utilities|IsValid (Variables|Default|GetTextbox_UI)
    (:Is%20Valid
      _)
    (:Is%20Not%20Valid
      (bind _returnvalue (UserInterface|CreateWidget "/Game/Player/UI/TextBox.TextBox_C" (Game|GetPlayerController 0)))))
  (bind _output_get (Variables|Default|SetTextbox_UI _returnvalue))
  (UserInterface|Viewport|AddtoViewport _output_get 0)
  (if (Variables|/Game/Player/UI/TextBox.TextBox_C|GetCanAdvance (Variables|Default|GetTextbox_UI))
    (bind _result (Math|Integer|IncrementInt (Variables|Default|GetTalkIndex))
      (:%20%20
        (if (< _result (Utilities|Array|Length (Variables|Default|GetContent)))
          (Default|PrintText (Variables|Default|GetTextbox_UI) (Utilities|Array|Get(acopy) (Variables|Default|GetContent) (Variables|Default|GetTalkIndex)))
          (else
            (CallFunction|Reset)))))))

(fn ConstructionScript)

(fn Reset
  (Widget|RemovefromParent (Variables|Default|GetTextbox_UI))
  (Variables|Default|SetTalkIndex -1)
  (Variables|Default|SetTextbox_UI 0))

(fn IsInteractable
  (return false))