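; NavTowerButton is an interactable button that sends a command to a referenced nav tower.
; OnInteract plays a timeline that lowers Sphere1 along its local Z axis as a press animation, then passes Command to NavTower via CustomActivateMessage when it finishes.
; It supplies a generic "interact" prompt, but IsInteractable always returns false.
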(event EventOnInteract
  (params (InteractingPlayer :type BP%20Sci%20Fi%20Player%20Character%20Object%20Reference))
  (bind _alpha (Timeline|Timeline PlayFromStart)
    (:Update
      (Transformation|SetRelativeLocation (Variables|Default|GetSphere1) (Math|Vector|Lerp(Vector) "0.000000,0.000000,25.000000" "0.000000,0.000000,10.000000" _alpha) false false))
    (:Finished
      (Class|BPIElectricity|CustomActivate(Message) (Variables|Default|GetNavTower) (Variables|Default|GetCommand)))))

(fn ConstructionScript)

(fn InteractPrompt
  (return "interact"))

(fn IsInteractable
  (return false))