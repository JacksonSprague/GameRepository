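; DoorSwitch is a switch Blueprint that toggles an On state and passes it to a linked door.
; OnInteract flips the flag, swaps the material on Sphere1 to match and calls OnSwitch on LinkedDoor with the new value.
; The construction script applies the matching material for the initial state.
; IsInteractable always returns false, even though the interact event is implemented.
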(event EventOnInteract
  (params (InteractingPlayer :type BP%20Sci%20Fi%20Player%20Character%20Object%20Reference))
  (if (Variables|Default|GetOn)
    (Variables|Default|SetOn false)
    (Rendering|Material|SetMaterial (Variables|Default|GetSphere1) 0 "/Engine/EngineMeshes/BackgroundMaterial.BackgroundMaterial")
    (else
      (Variables|Default|SetOn true)
      (Rendering|Material|SetMaterial (Variables|Default|GetSphere1) 0 "/Engine/MapTemplates/Materials/BasicAsset03.BasicAsset03")))
  (Default|OnSwitch (Variables|Default|GetLinkedDoor) (Variables|Default|GetOn)))

(fn ConstructionScript
  (if (Variables|Default|GetOn)
    (Rendering|Material|SetMaterial (Variables|Default|GetSphere1) 0 "/Engine/MapTemplates/Materials/BasicAsset03.BasicAsset03")
    (else
      (Rendering|Material|SetMaterial (Variables|Default|GetSphere1) 0 "/Engine/EngineMeshes/BackgroundMaterial.BackgroundMaterial"))))

(fn IsInteractable
  (return false))